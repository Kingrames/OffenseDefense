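; StartLight is an interactable light actor that the player can switch on or off by pressing E while nearby.
; Entering its trigger volume enables input and toggles a helpful message; leaving disables input and toggles the message again.
; The E key toggles both a spot light and a point light.
; The construction script applies a configurable color and default on/off state to both lights.
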(event `self.TriggerVolume.OnComponentBeginOverlap`
  (params (OtherActor :type "Actor Object Reference") (OtherComp :type "PrimitiveComponent Object Reference") (OtherBodyIndex :type Integer))
  ;[0.5969 0.8002 1] When we enter the trigger volume, enable input and show the helpful message. Disable upon exit
  (`self.EnableInput` (`GameplayStatics.GetPlayerController` 0))
  (`SceneComponent.ToggleVisibility` (`self.HelpfulMessage`) false :!label _label))

(event `self.TriggerVolume.OnComponentEndOverlap`
  (params (OtherActor :type "Actor Object Reference") (OtherComp :type "PrimitiveComponent Object Reference") (OtherBodyIndex :type Integer))
  ;[0.5969 0.8002 1] When we enter the trigger volume, enable input and show the helpful message. Disable upon exit
  (`self.DisableInput` (`GameplayStatics.GetPlayerController` 0))
  (goto _label))

(event `Key|E`
  ;[1 0.6658 0.5002] Hit E to turn on the light
  (:`Pressed`
    (`SceneComponent.ToggleVisibility` (`self.StartLightSpotLight`) false)
    (`SceneComponent.ToggleVisibility` (`self.StartLightPointLight`) false)))

(fn `UserConstructionScript`
  (`LightComponent.SetLightColor` (`self.StartLightPointLight`) (`self.LightColor`))
  (`LightComponent.SetLightColor` (`self.StartLightSpotLight`) (`self.LightColor`))
  (`SceneComponent.SetVisibility` (`self.StartLightSpotLight`) (`self.EnabledByDefault`) false)
  (`SceneComponent.SetVisibility` (`self.StartLightPointLight`) (`self.EnabledByDefault`) false))